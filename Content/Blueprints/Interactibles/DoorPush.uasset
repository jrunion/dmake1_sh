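; DoorPush is an interactible door that swings open when a Character walks into a trigger on either side.
; Front and Back overlap volumes each play their own timeline, which sets the yaw of a Pivot component.
; Leaving a volume reverses that side's timeline from its end after a one-second delay.
; Per-side overlap flags are set but never read, so nothing guards the two timelines against each other.
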(event `self.Front.OnComponentBeginOverlap`
  (params (OverlappedComponent :type "PrimitiveComponent Object Reference") (OtherActor :type "Actor Object Reference") (OtherComp :type "PrimitiveComponent Object Reference") (OtherBodyIndex :type Integer) (bFromSweep :type Boolean) (SweepResult :type "HitResult Structure (by ref)"))
  ;[1 1 1] Front Controls
  (cast `Character` OtherActor)
  (set `self.overlappedF` true)
  (bind (_direction _newtrack_0) (`Timeline|Timeline_0` :!via `PlayFromStart` :!label _label)
    (:`Update`
      (`SceneComponent.K2_SetRelativeRotation` (`self.pivot`) (`KismetMathLibrary.MakeRotator` 0.0 0.0 _newtrack_0) false false))))

(event `self.Front.OnComponentEndOverlap`
  (params (OverlappedComponent :type "PrimitiveComponent Object Reference") (OtherActor :type "Actor Object Reference") (OtherComp :type "PrimitiveComponent Object Reference") (OtherBodyIndex :type Integer))
  ;[1 1 1] Front Controls
  (cast `Character` OtherActor)
  (set `self.overlappedF` false)
  (`KismetSystemLibrary.Delay` 1.0)
  (goto _label :!via `ReverseFromEnd`))

(event `self.Back.OnComponentBeginOverlap`
  (params (OverlappedComponent :type "PrimitiveComponent Object Reference") (OtherActor :type "Actor Object Reference") (OtherComp :type "PrimitiveComponent Object Reference") (OtherBodyIndex :type Integer) (bFromSweep :type Boolean) (SweepResult :type "HitResult Structure (by ref)"))
  ;[1 1 1] BackControls
  (cast `Character` OtherActor)
  (set `self.overlappedB` true)
  (bind (_direction _newtrack_0) (`Timeline|Timeline_1` :!via `PlayFromStart` :!label _label_2)
    (:`Update`
      (`SceneComponent.K2_SetRelativeRotation` (`self.pivot`) (`KismetMathLibrary.MakeRotator` 0.0 0.0 _newtrack_0) false false))))

(event `self.Back.OnComponentEndOverlap`
  (params (OverlappedComponent :type "PrimitiveComponent Object Reference") (OtherActor :type "Actor Object Reference") (OtherComp :type "PrimitiveComponent Object Reference") (OtherBodyIndex :type Integer))
  ;[1 1 1] BackControls
  (cast `Character` OtherActor)
  (set `self.overlappedB` false)
  (`KismetSystemLibrary.Delay` 1.0)
  (goto _label_2 :!via `ReverseFromEnd`))

(fn `UserConstructionScript`)