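; DoorPush_L is an interactible push door that toggles open and closed when the player interacts with it.
; The construction script starts it closed, and PlayerInteractedwith flips the Closed and Opened flags while playing or reversing a timeline.
; On each update, the timeline track sets the yaw of the Pivot component to swing the door.
; A separate MoveDoor function holds partly disconnected front-overlap state logic and is not called in this graph.
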(event `self.Player_Interacted_With`
  ;[1 1 1] Front Controls
  (if (`self.Closed`)
    (set `self.Closed` false)
    (set `self.Opened` true)
    (bind (_direction _newtrack_0) (`Timeline|Timeline_0` :!label _label)
      (:`Update`
        (`SceneComponent.K2_SetRelativeRotation` (`self.pivot`) (`KismetMathLibrary.MakeRotator` 0.0 0.0 _newtrack_0) false false)))
    (elif (`self.Opened`)
      (set `self.Closed` true)
      (set `self.Opened` false)
      (goto _label :!via `Reverse`))))

(fn `MoveDoor`
  ;[1 1 1] Front Controls
  (if true
    (if (`self.overlappedF`)
      (set `self.OpeningF` true)
      (if (`self.Closed`)
        (set `self.Closed` false)
        (elif (`self.Opened`)
          (set `self.Closed` true)
          (elif true
            (set `self.Closed` true)))))))

(fn `UserConstructionScript`
  (set `self.Closed` true)
  (set `self.Opened` false))