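; Interactible light switch that turns on a group of tagged Spotlight actors.
; The construction script caches all Spotlights with the configured tag and sets them to a starting brightness.
; Interact raises the cached lights to the target brightness and sets a flag, so it works only once, with no path to switch them off.
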(event `/Game/Blueprints/Interactibles/Interactable.Interact`
  ;[1 1 1] Lights Turn on
  (if (not (`self.LightOn?`))
    (for _array_element (`self.LightObjects`)
      (`LightComponent.SetIntensity` (`Light.LightComponent` _array_element) (`self.Brightness`))
      (set `self.LightOn?` true))))

(fn `UserConstructionScript`
  (`parent.UserConstructionScript`)
  (bind _outactors (`GameplayStatics.GetAllActorsOfClassWithTag` "/Game/Blueprints/Spotlight.Spotlight_C" (`self.TagName`)))
  (bind _output_get (set `self.LightObjects` _outactors))
  (for _array_element _output_get
    (`LightComponent.SetIntensity` (`SpotLight.SpotLightComponent` _array_element) (`self.StartBrightness`))))