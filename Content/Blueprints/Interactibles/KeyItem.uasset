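; Pickup actor for a key item that the player collects by interacting with it.
; On Interact, it casts the first player pawn to BP_Player, adds its ItemName to that player's Inventory, prints the name and destroys itself.
; An unconnected node would derive ItemName from the object's name, so the graph uses the variable's existing value.
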(event `/Game/Blueprints/Interactibles/Interactable.Interact`
  (bind _itemname (`self.ItemName`))
  ;[1 1 1] Stuff
  (bind _asbp_player (cast `/Game/Blueprints/BP_Player` (`GameplayStatics.GetPlayerPawn` 0)))
  (`/Game/Blueprints/Components/Inventory.Add Item` (`/Game/Blueprints/BP_Player.Inventory` _asbp_player) _itemname)
  (`KismetSystemLibrary.PrintString` _itemname)
  (`KismetSystemLibrary.PrintString` _itemname)
  (`self.K2_DestroyActor`))

(fn `UserConstructionScript`)