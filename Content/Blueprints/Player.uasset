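; Player Blueprint that handles movement and spring-arm camera control from axis inputs.
; Forward/back and right/left inputs add movement along directions derived from control yaw only, ignoring pitch and roll.
; Horizontal camera input drives controller yaw, while vertical input rotates the SpringArm directly.
; The arm's target pitch is then clamped to a fixed range and written back as relative rotation with zero yaw and roll.
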(event `InputAxis|Camera: Right/Left`
  (params (AxisValue :type "Float (single-precision)"))
  ;[1 1 1] Camera Movement : x-Axis
  (`self.AddControllerYawInput` AxisValue))

(event `InputAxis|Movment: Forward/Back`
  (params (AxisValue :type "Float (single-precision)"))
  ;[1 1 1] Player Movement
  (`self.AddMovementInput` (`KismetMathLibrary.GetForwardVector` (`KismetMathLibrary.MakeRotator` 0.0 0.0 (.yaw (`self.GetControlRotation`)))) AxisValue))

(event `InputAxis|Camera: Up/ Down`
  (params (AxisValue :type "Float (single-precision)"))
  ;[1 1 1] Camera Movement : Y-Axis
  (`SceneComponent.K2_AddLocalRotation` (`self.SpringArm`) (`KismetMathLibrary.MakeRotator` 0.0 AxisValue) false false)
  (`SceneComponent.K2_SetRelativeRotation` (`self.SpringArm`) (`KismetMathLibrary.MakeRotator` 0.0 (`KismetMathLibrary.ClampAngle` (.pitch (`SpringArmComponent.GetTargetRotation` (`self.SpringArm`))) -60.0 20.0)) false false))

(event `InputAxis|Movment: Right/Left`
  (params (AxisValue :type "Float (single-precision)"))
  ;[1 1 1] Player Movement
  (`self.AddMovementInput` (`KismetMathLibrary.GetRightVector` (`KismetMathLibrary.MakeRotator` 0.0 0.0 (.yaw (`self.GetControlRotation`)))) AxisValue))

(fn `UserConstructionScript`)