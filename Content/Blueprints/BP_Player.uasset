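; BP_Player is the player Blueprint, handling movement, camera look, running, interaction and an inventory debug printout.
; Axis inputs move relative to control rotation; the run button raises a Speed multiplier that scales only forward/back input.
; Each tick, a short debug-drawn visibility trace from the capsule caches any hit actor implementing Interactable.
; Interact sends InteractMessage to that cached actor, while Check Inventory prints the item count and entries.
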(event `InputAction|Buttond: Check Inventory`
  (params (Key :type "Key Structure"))
  (bind _inventory (`/Game/Blueprints/Components/Inventory.inventory` (`self.Inventory`)))
  ; Inventory
  (:`Pressed`
    (`KismetSystemLibrary.PrintString` (`KismetStringLibrary.Conv_IntToString` (`KismetArrayLibrary.Array_Length` _inventory)))
    (for _array_element _inventory
      (`KismetSystemLibrary.PrintString` _array_element))))

(event `InputAction|Buttons: Run`
  (params (Key :type "Key Structure"))
  ;[1 1 1] Running
  (:`Pressed`
    (set `self.Speed` 1000.0))
  (:`Released`
    (set `self.Speed` 1.0)))

(event `InputAxis|Camera: Up/ Down`
  (params (AxisValue :type "Float (single-precision)"))
  ;[0.4907 0.04116 1] Camera Movement
  (`self.AddControllerPitchInput` AxisValue))

(event `InputAxis|Movment: Forward/Back`
  (params (AxisValue :type "Float (single-precision)"))
  ;[1 0.05535 0.8201] Movement
  (`self.AddMovementInput` (`KismetMathLibrary.GetForwardVector` (`self.GetControlRotation`)) (* AxisValue (`self.Speed`))))

(event `InputAxis|Camera: Right/Left`
  (params (AxisValue :type "Float (single-precision)"))
  ;[0.4907 0.04116 1] Camera Movement
  (`self.AddControllerYawInput` AxisValue))

(event `InputAxis|Movment: Right/Left`
  (params (AxisValue :type "Float (single-precision)"))
  ;[1 0.05535 0.8201] Movement
  (`self.AddMovementInput` (`KismetMathLibrary.GetRightVector` (`self.GetControlRotation`)) AxisValue))

(event `InputAction|Buttons: Interact`
  (params (Key :type "Key Structure"))
  ;[1 1 1] interaction
  (:`Pressed`
    (message `/Game/Blueprints/Interactibles/Interactable.Interact` (stale `self.ReceiveTick` _output_get))))

(event `self.ReceiveTick`
  (params (DeltaSeconds :type "Float (single-precision)"))
  (bind _capsulecomponent (`self.CapsuleComponent`))
  (bind _returnvalue (`SceneComponent.K2_GetComponentLocation` _capsulecomponent))
  ;[1 1 1] Raytrace: Detect Object
  (bind _outhit (`KismetSystemLibrary.LineTraceSingle` :`Start` _returnvalue :`End` (+ _returnvalue (* (`KismetMathLibrary.GetForwardVector` (`SceneComponent.K2_GetComponentRotation` _capsulecomponent)) 150.0)) :`TraceChannel` "TraceTypeQuery1" :`DrawDebugType` "ForOneFrame"))
  (bind (_bblockinghit _binitialoverlap _time _distance _location _impactpoint _normal _impactnormal _physmat _hitactor) (`GameplayStatics.BreakHitResult` _outhit))
  ;[1 1 1] interaction
  (if _bblockinghit
    (if (`KismetSystemLibrary.DoesImplementInterface` _hitactor "/Game/Blueprints/Interactibles/Interactable.Interactable_C")
      (bind _output_get (set `self.IntActor` _hitactor))
      (else
        (set `self.IntActor` null :!label _label)))
    (else
      (goto _label))))

(fn `UserConstructionScript`
  (set `self.Speed` 1.0))